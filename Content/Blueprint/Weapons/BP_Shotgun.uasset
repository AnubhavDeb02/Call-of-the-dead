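; Shotgun weapon Blueprint that extends a parent weapon class with shotgun-specific ammo, firing effects and reload timing.
; On BeginPlay it pulls ShotgunAmmoData from FPS_gameInstance and derives reload time from magazine capacity.
; Firing runs the parent logic, then plays the gun mesh fire animation and spawns a shell emitter at the AmmoEject socket.
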(event `self.ReceiveBeginPlay`
  (`parent.ReceiveBeginPlay`)
  (bind _asfps_game_instance (cast `/Game/Blueprint/FPS_gameInstance` (`GameplayStatics.GetGameInstance`)))
  (set `self.ammoData` (`/Game/Blueprint/FPS_gameInstance.shotgunAmmoData` _asfps_game_instance))
  (`self.SetReloadTime`))

(event `self.weaponFire`
  (params (fireType :type "/Game/Blueprint/Enums/FireType Enum" :default "NewEnumerator0"))
  (bind (_returnvalue_location _returnvalue_rotation) (`KismetMathLibrary.BreakTransform` (`SceneComponent.GetSocketTransform` (`self.GunMesh`) "AmmoEject" "RTS_World")))
  (`parent.weaponFire` fireType)
  (`SkeletalMeshComponent.PlayAnimation` (`self.GunMesh`) "/Game/MilitaryWeapDark/Weapons/Anims/Fire_Shotgun_W.Fire_Shotgun_W" false)
  (`GameplayStatics.SpawnEmitterAtLocation` "/Game/Particles/FX_shotgunShell.FX_shotgunShell" _returnvalue_location _returnvalue_rotation))

(event `SetReloadTime`
  (set `self.reloadTime` (* (`self.maxMagAmmo`) 0.5)))

(fn `UserConstructionScript`
  (`parent.UserConstructionScript`))