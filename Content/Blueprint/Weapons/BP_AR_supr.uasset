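; Suppressed assault rifle weapon Blueprint, a child of a shared weapon class, that pulls its ammo data from the FPS game instance on BeginPlay.
; WeaponFire shoots immediately and starts a looping timer at the auto-fire rate, which StopFire clears.
; Each shot, gated by the auto-rifle flag, runs parent fire logic, plays the gun animation and notifies the player, stopping and reloading when ammo runs out.
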(event `self.ReceiveBeginPlay`
  (`parent.ReceiveBeginPlay`)
  (bind _asfps_game_instance (cast `/Game/Blueprint/FPS_gameInstance` (`GameplayStatics.GetGameInstance`)))
  (set `self.ammoData` (`/Game/Blueprint/FPS_gameInstance.arSuprAmmoData` _asfps_game_instance)))

(event `self.weaponFire`
  (params (fireType :type "/Game/Blueprint/Enums/FireType Enum" :default "NewEnumerator0"))
  (set `self.isRifleFiring?` true)
  (`self.RifleFire`)
  (bind _returnvalue (`KismetSystemLibrary.K2_SetTimerDelegate` (delegate `RifleFire`) (`self.AutoFireRate`) true))
  (set `self.RifleFireTimerHandle` _returnvalue))

(event `RifleFire`
  (if (`self.isAutoRifle?`)
    (`parent.weaponFire` (stale `self.weaponFire` fireType))
    (`SkeletalMeshComponent.PlayAnimation` (`self.GunMesh`) "/Game/MilitaryWeapDark/Weapons/Anims/Fire_Rifle_W.Fire_Rifle_W" false)
    (`/Game/Blueprint/FPS_character.characterFireWeapon` (`self.player ref`) "NewEnumerator13")
    (if (<= (`self.currentAmmo`) 0)
      (`self.stopFire`)
      (`/Game/Blueprint/FPS_character.reload` (`self.player ref`)))))

(event `self.stopFire`
  (`parent.stopFire`)
  (set `self.isRifleFiring?` false)
  (`KismetSystemLibrary.K2_ClearAndInvalidateTimerHandle` (`self.RifleFireTimerHandle`)))

(fn `UserConstructionScript`
  (`parent.UserConstructionScript`))