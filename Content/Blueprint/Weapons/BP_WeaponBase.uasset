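; Base weapon Blueprint for an FPS, handling firing, magazine and reserve ammo, reload and recoil.
; WeaponFire uses CalculateShot's camera trace, spread unless aiming a non-pistol, for single or multi-bullet hitscan damage and impacts, or projectiles launched from the muzzle socket toward the hit.
; Auto rifles add timeline-driven camera kick with random yaw, then reverse it.
; Player aim events set IsAiming, and Tick calls the player's AdsFOV.
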(event `self.ReceiveBeginPlay`
  (bind _asfps_character (cast `/Game/Blueprint/FPS_character` (`GameplayStatics.GetPlayerPawn` 0)))
  (set `self.player ref` _asfps_character)
  (add `/Game/Blueprint/FPS_character.aimEnter` _asfps_character (delegate `onAimEnter`))
  (add `/Game/Blueprint/FPS_character.aimExit` _asfps_character (delegate `onAimExit`)))

(event `onAimEnter`
  (set `self.isAiming?` true))

(event `onAimExit`
  (set `self.isAiming?` false))

(event `AutoRecoil`
  (bind _returnvalue (`GameplayStatics.GetPlayerPawn` 0))
  (bind (_direction _alpha) (`Timeline|RecoilTimeline` :!via `PlayFromStart` :!label _label)
    (:`Update`
      (switch `ETimelineDirection` _direction
        (:`Forward`
          (bind _returnvalue_2 (`KismetMathLibrary.Lerp` 0.0 (`self.recoilPitch`) _alpha))
          (`Pawn.AddControllerPitchInput` _returnvalue _returnvalue_2)
          (`Pawn.AddControllerYawInput` _returnvalue (`KismetMathLibrary.RandomFloatInRange` -0.05 0.05)))
        (:`Backward`
          (`Pawn.AddControllerPitchInput` _returnvalue (* _returnvalue_2 -1.0)))))
    (:`Finished`
      (`self.ReverseRecoil`)
      (`KismetSystemLibrary.RetriggerableDelay` 0.05)
      (`self.StopRecoil`))))

(event `StopRecoil`
  (goto _label :!via `Stop`))

(event `ReverseRecoil`
  (goto _label :!via `Reverse`))

(event `self.ReceiveTick`
  (params (DeltaSeconds :type "Float (single-precision)"))
  (`/Game/Blueprint/FPS_character.adsFOV` (`self.player ref`)))

(fn `addDamage`
  (params (hitResult :type "HitResult Structure"))
  (message `/Game/Blueprint/Interfaces/TakeDamage.TakeDamage` (`.HitActor` (`GameplayStatics.BreakHitResult` hitResult)) (`self.ammoData`) (`self.criticalHitDamageModifier`) hitResult))

(fn `calculateShot`
  (params (Camera :type "CameraComponent Object Reference") (WeaponMesh :type "SceneComponent Object Reference") (`Weapon Fire Socket Name` :type Name))
  (returns (`Hit Result` :type "HitResult Structure") (projectileTransform :type "Transform Structure"))
  (locals (`Local Camera` :type "CameraComponent Object Reference") (`Local Weapon Mesh` :type "SceneComponent Object Reference") (`Local Socket Name` :type Name) (`Local Projectile Transform` :type "Transform Structure"))
  (bind _bulletspread (`self.bulletSpread`))
  (bind (_returnvalue_location _returnvalue_rotation) (`KismetMathLibrary.BreakTransform` (`SceneComponent.K2_GetComponentToWorld` (`local.Local Camera`))))
  (bind _returnvalue (`SceneComponent.GetSocketLocation` (`local.Local Weapon Mesh`) (`local.Local Socket Name`)))
  (bind _returnvalue_2 (* _bulletspread -1.0))
  (bind _returnvalue_3 (+ _returnvalue_location (* (`KismetMathLibrary.GetForwardVector` _returnvalue_rotation) 10000.0)))
  (`|ExecutionSequence`
    (:`then_0`
      (set `local.Local Camera` Camera)
      (set `local.Local Weapon Mesh` WeaponMesh)
      (set `local.Local Socket Name` `Weapon Fire Socket Name`))
    (:`then_1`
      (bind (_outhit _returnvalue_4) (`KismetSystemLibrary.LineTraceSingleForObjects` _returnvalue_location (select `bool` (and (`self.isAiming?`) (not (`self.isPistol?`))) :`false` (`KismetMathLibrary.MakeVector` (+ (.x _returnvalue_3) (`KismetMathLibrary.RandomFloatInRange` _returnvalue_2 _bulletspread)) (+ (.y _returnvalue_3) (`KismetMathLibrary.RandomFloatInRange` _returnvalue_2 _bulletspread)) (+ (.z _returnvalue_3) (`KismetMathLibrary.RandomFloatInRange` _returnvalue_2 _bulletspread))) :`true` _returnvalue_3) (`|MakeArray` "ObjectTypeQuery1" "ObjectTypeQuery2" :!type "EObjectTypeQuery Enum") false (`|MakeArray` (`GameplayStatics.GetPlayerPawn` 0) :!type "Actor Object Reference")))
      (if _returnvalue_4
        (set `local.Local Projectile Transform` (`KismetMathLibrary.MakeTransform` _returnvalue (`KismetMathLibrary.FindLookAtRotation` _returnvalue (`.ImpactPoint` (`GameplayStatics.BreakHitResult` _outhit)))))
        (else
          (set `local.Local Projectile Transform` (`KismetMathLibrary.MakeTransform` _returnvalue (`Pawn.GetControlRotation` (cast `Pawn` (`ActorComponent.GetOwner` (`local.Local Camera`)) :!pure true)))))))
    (:`then_2`
      (return _outhit (`local.Local Projectile Transform`)))))

(fn `hasAmmoInMag`
  (returns (`has Ammo` :type Boolean) (`mag Full` :type Boolean))
  (return (> (`self.currentAmmo`) 0) (== (`self.currentAmmo`) (`self.maxMagAmmo`))))

(fn `hasExtraAmmo`
  (returns (`have Extra Ammo` :type Boolean))
  (return (> (`self.totalCurrentAmmo`) 0)))

(fn `stopFire`)

(fn `UserConstructionScript`)

(fn `weaponFire`
  (params (fireType :type "/Game/Blueprint/Enums/FireType Enum" :default "NewEnumerator0"))
  (set `self.currentAmmo` (- (`self.currentAmmo`) 1))
  (switch `/Game/Blueprint/Enums/FireType` fireType
    (:`NewEnumerator0`
      (if (`self.multipleBullets?`)
        (for _ (range (`self.bulletCount`))
          (bind _hit_result (`self.calculateShot` (`/Game/Blueprint/FPS_character.Camera` (`self.player ref`)) (`self.GunMesh`) (`self.muzzleSocketName`) :!label _label))
          (bind (_bblockinghit _binitialoverlap _time _distance _location _impactpoint) (`GameplayStatics.BreakHitResult` _hit_result))
          (`|SpawnActorFromClass` (`self.impactEffectClass`) (`KismetMathLibrary.MakeTransform` _impactpoint) "Undefined" "OverrideRootScale" null _hit_result _bblockinghit null)
          (`self.addDamage` _hit_result)
          (if (`self.isAutoRifle?`) :!label _label_2
            (`self.AutoRecoil`)))
        (else
          (goto _label))))
    (:`NewEnumerator1`
      (bind (_hit_result_2 _projectiletransform) (`self.calculateShot` (`/Game/Blueprint/FPS_character.Camera` (`self.player ref`)) (`self.GunMesh`) (`self.muzzleSocketName`)))
      (bind _returnvalue (`|SpawnActorFromClass` (`self.projectile`) _projectiletransform "AlwaysSpawn" "OverrideRootScale" null (`self.ammoData`) (`self.criticalHitDamageModifier`) null))
      (set `self.spawnProjectile` _returnvalue)
      (goto _label_2))))

(fn `weaponReload`
  (bind _maxmagammo (`self.maxMagAmmo`))
  (bind _totalcurrentammo (`self.totalCurrentAmmo`))
  (bind _currentammo (`self.currentAmmo`))
  (if (> _totalcurrentammo _maxmagammo)
    (set `self.totalCurrentAmmo` (- _totalcurrentammo (- _maxmagammo _currentammo)))
    (set `self.currentAmmo` _maxmagammo)
    (elif (< (+ _totalcurrentammo _currentammo) _maxmagammo)
      (set `self.currentAmmo` (+ _currentammo _totalcurrentammo))
      (set `self.totalCurrentAmmo` 0)
      (else
        (set `self.totalCurrentAmmo` (- _totalcurrentammo (- _maxmagammo _currentammo)))
        (set `self.currentAmmo` _maxmagammo)))))