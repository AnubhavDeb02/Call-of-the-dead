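; Sniper rifle child weapon that adds a full-screen scope view when aiming.
; BeginPlay loads its ammo data from the game instance, and firing plays the gun animation and ejects a shell particle at the AmmoEject socket.
; Aiming in blocks weapon switching and reloading, then after a short delay shows the scope widget while hiding the gun, player pawn and main HUD.
; Aiming out reverses these changes.
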(event `self.ReceiveBeginPlay`
  (`parent.ReceiveBeginPlay`)
  (bind _asfps_game_instance (cast `/Game/Blueprint/FPS_gameInstance` (`GameplayStatics.GetGameInstance`)))
  (set `self.ammoData` (`/Game/Blueprint/FPS_gameInstance.sniperAmmoData` _asfps_game_instance)))

(event `self.weaponFire`
  (params (fireType :type "/Game/Blueprint/Enums/FireType Enum" :default "NewEnumerator0"))
  (bind (_returnvalue_location _returnvalue_rotation) (`KismetMathLibrary.BreakTransform` (`SceneComponent.GetSocketTransform` (`self.GunMesh`) "AmmoEject" "RTS_World")))
  (`parent.weaponFire` fireType)
  (`SkeletalMeshComponent.PlayAnimation` (`self.GunMesh`) "/Game/MilitaryWeapSilver/Weapons/Animations/Fire_SniperRifle_W.Fire_SniperRifle_W" false)
  (`GameplayStatics.SpawnEmitterAtLocation` "/Game/Particles/FX_sniperShell.FX_sniperShell" _returnvalue_location _returnvalue_rotation))

(event `self.onAimEnter`
  (bind _player_ref (`self.player ref`))
  (bind _sniperscoperef (`/Game/Blueprint/FPS_character.SniperScopeRef` (`self.player ref`)))
  (`parent.onAimEnter`)
  (if (== (`/Game/Blueprint/FPS_character.currentWeapon` (`self.player ref`)) self)
    (set `/Game/Blueprint/FPS_character.canSwitchWeapon?` false _player_ref)
    (set `/Game/Blueprint/FPS_character.canReload?` false _player_ref)
    (`KismetSystemLibrary.Delay` 0.1)
    (if (not (`Widget.IsInViewport` _sniperscoperef))
      (`UserWidget.AddToViewport` _sniperscoperef 0)
      (`SceneComponent.SetHiddenInGame` (`self.GunMesh`) true false)
      (`self.SetActorHiddenInGame` (`GameplayStatics.GetPlayerPawn` 0) true)
      (`Widget.SetVisibility` (`/Game/Blueprint/FPS_character.mainHUDRef` (`self.player ref`)) "Collapsed"))))

(event `self.onAimExit`
  (bind _player_ref (`self.player ref`))
  (`parent.onAimExit`)
  (set `/Game/Blueprint/FPS_character.canSwitchWeapon?` true _player_ref)
  (set `/Game/Blueprint/FPS_character.canReload?` true _player_ref)
  (`Widget.RemoveFromParent` (`/Game/Blueprint/FPS_character.SniperScopeRef` _player_ref))
  (`SceneComponent.SetHiddenInGame` (`self.GunMesh`) false false)
  (`self.SetActorHiddenInGame` (`GameplayStatics.GetPlayerPawn` 0) false)
  (`Widget.SetVisibility` (`/Game/Blueprint/FPS_character.mainHUDRef` (`self.player ref`)) "Visible"))

(fn `UserConstructionScript`
  (`parent.UserConstructionScript`))