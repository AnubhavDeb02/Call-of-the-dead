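; FPS_controller is a controller Blueprint that turns mouse input into yaw and pitch for the first-person player.
; On BeginPlay it stores the FPS_character pawn and caches whether its current weapon is a pistol, with no later refresh in this file.
; Both mouse axes halve their input while the character aims in one specific weapon state, unless that cached pistol flag is set.
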(event `self.ReceiveBeginPlay`
  (bind _asfps_character (cast `/Game/Blueprint/FPS_character` (`GameplayStatics.GetPlayerPawn` 0)))
  (bind _output_get (set `self.playerRef` _asfps_character))
  (bind _currentweapon (`/Game/Blueprint/FPS_character.currentWeapon` _output_get))
  (`/Engine/EditorBlueprintResources/StandardMacros.IsValid` _currentweapon
    (:`Is Valid`
      (set `self.isPistol?` (`/Game/Blueprint/Weapons/BP_WeaponBase.isPistol?` _currentweapon)))))

(event `InputAxis|mouseX`
  (params (AxisValue :type "Float (single-precision)"))
  (bind _playerref (`self.playerRef`))
  (`self.AddYawInput` (select `bool` (and (`/Game/Blueprint/FPS_character.isAiming?` _playerref) (`|EnumEquality` (`/Game/Blueprint/FPS_character.hasWeaponEnum` _playerref) "NewEnumerator1") (not (`self.isPistol?`))) :`false` AxisValue :`true` (/ AxisValue 2.0) :!type "Float (single-precision)")))

(event `InputAxis|mouseY`
  (params (AxisValue :type "Float (single-precision)"))
  (bind _playerref (`self.playerRef`))
  (`self.AddPitchInput` (select `bool` (and (`/Game/Blueprint/FPS_character.isAiming?` _playerref) (`|EnumEquality` (`/Game/Blueprint/FPS_character.hasWeaponEnum` _playerref) "NewEnumerator1") (not (`self.isPistol?`))) :`false` AxisValue :`true` (/ AxisValue 2.0) :!type "Float (single-precision)")))

(fn `UserConstructionScript`)