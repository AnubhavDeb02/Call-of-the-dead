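; AI controller that runs a behavior tree and passes perception results to its blackboard.
; On each perception update it reads the last sensed stimuli of every updated actor.
; The AIsense function switches on stimulus array index rather than sense class, writing index 0's success flag to the canSeePlayer key.
; Other indices are unhandled, and no check confirms the sensed actor is the player.
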(event `self.ReceiveBeginPlay`
  (`self.RunBehaviorTree` "/Game/Blueprint/AI/AI_BehaviorTree.AI_BehaviorTree"))

(event `self.AIPerception.OnPerceptionUpdated`
  (params (UpdatedActors :type "Array of Actor Object Reference (by ref)"))
  (for _array_element UpdatedActors
    (bind _info (`AIPerceptionComponent.GetActorsPerception` (`self.AIPerception`) _array_element))
    (`self.AIsense` (`.LastSensedStimuli` (break `ActorPerceptionBlueprintInfo` _info)))))

(fn `AIsense`
  (params (`AI Stimulus` :type "Array of AIStimulus Structure"))
  (locals (currentSense :type "AIStimulus Structure"))
  (for (_array_element _array_index) `AI Stimulus`
    (set `local.currentSense` _array_element)
    (switch `int` _array_index
      (:`0`
        (`BlackboardComponent.SetValueAsBool` (`AIBlueprintHelperLibrary.GetBlackboard` null) "canSeePlayer" (`.bSuccessfullySensed` (break `AIStimulus` (`local.currentSense`))))))))

(fn `UserConstructionScript`)