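; AI character that takes weapon hits, tracks health and ragdolls on death.
; TakeDamage feeds ammo damage through SetDamage, which always applies the critical multiplier despite rolling for crits, then scales by the physical material's DestructibleDamageThresholdScale.
; UpdateHealth flags death, triggering mesh physics with a weapon-based impulse away from the player and removing the capsule.
; Each hit shows randomly offset floating damage and replaces the hitmarker widget.
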(event `self.ReceiveBeginPlay`
  (bind _asfps_character (cast `/Game/Blueprint/FPS_character` (`GameplayStatics.GetPlayerPawn` 0)))
  (set `self.characterRef` _asfps_character))

(event `self.Floating Damage`
  (params (damage :type "Float (double-precision)") (`impact Point` :type "Vector Structure"))
  (bind (_x _y) (`KismetMathLibrary.BreakVector2D` (`WidgetLayoutLibrary.ProjectWorldLocationToWidgetPosition` (`GameplayStatics.GetPlayerController` 0) `impact Point`)))
  (bind _returnvalue (`|CreateWidget` "/Game/Blueprint/UMG/UI_FloatingDamage.UI_FloatingDamage_C" null damage))
  (`Widget.SetRenderTranslation` (`/Game/Blueprint/UMG/UI_FloatingDamage.screenPositionSizeBox` _returnvalue) (`KismetMathLibrary.MakeVector2D` (+ (+ _x -50.0) (`KismetMathLibrary.RandomFloatInRange` -25.0 25.0)) (+ (+ _y -100.0) (`KismetMathLibrary.RandomFloatInRange` -10.0 10.0))))
  (`UserWidget.AddToViewport` _returnvalue 0))

(event `/Game/Blueprint/Interfaces/TakeDamage.TakeDamage`
  (params (AmmoDara :type "/Game/Blueprint/Structs/AmmoData Structure") (CriticalHitModifier :type "Float (double-precision)") (HitResult :type "HitResult Structure"))
  (bind (_damage _criticalhitchance) (break `/Game/Blueprint/Structs/AmmoData` AmmoDara))
  (bind (_bblockinghit _binitialoverlap _time _distance _location _impactpoint _normal _impactnormal _physmat _hitactor _hitcomponent _hitbonename _bonename) (`GameplayStatics.BreakHitResult` HitResult))
  (bind _hitmarkerref (`self.hitmarkerRef`))
  (bind _damagetoapply (`self.setDamage` _damage _criticalhitchance CriticalHitModifier HitResult))
  (`KismetSystemLibrary.PrintString` (`KismetStringLibrary.Conv_DoubleToString` _damagetoapply))
  (bind _isdead_ (`self.updateHealth` _damagetoapply))
  (bind _output_get (set `self.isDead?` _isdead_))
  (if _output_get
    (`self.death` _impactpoint _bonename))
  (`self.Floating Damage` _damagetoapply _impactpoint)
  (`/Engine/EditorBlueprintResources/StandardMacros.IsValid` _hitmarkerref
    (:`Is Valid`
      (`Widget.RemoveFromParent` _hitmarkerref))
    (:`Is Not Valid`
      _))
  (bind _returnvalue (`|CreateWidget` "/Game/Blueprint/UMG/UI_Hitmarker.UI_Hitmarker_C" null (`self.isDead?`)))
  (bind _output_get_2 (set `self.hitmarkerRef` _returnvalue))
  (`UserWidget.AddToViewport` _output_get_2 0))

(fn `death`
  (params (impactPoint :type "Vector Structure") (boneName :type Name))
  (bind _mesh (`self.Mesh`))
  (bind _characterref (`self.characterRef`))
  (bind _capsulecomponent (`self.CapsuleComponent`))
  (`PrimitiveComponent.SetSimulatePhysics` _mesh true)
  (`PrimitiveComponent.AddImpulseAtLocation` _mesh (* (`KismetMathLibrary.GetDirectionUnitVector` (`self.K2_GetActorLocation` _characterref) (`self.K2_GetActorLocation`)) (select `/Game/Blueprint/Enums/hasWeapon` (`/Game/Blueprint/FPS_character.hasWeaponEnum` _characterref) :`NewEnumerator0` (`KismetMathLibrary.Conv_DoubleToVector` (`self.defaultKillImpulse`)) :`NewEnumerator1` (`KismetMathLibrary.Conv_DoubleToVector` (`/Game/Blueprint/Weapons/BP_WeaponBase.killImpulse` (`/Game/Blueprint/FPS_character.currentWeapon` _characterref))))) impactPoint boneName)
  (`/Engine/EditorBlueprintResources/StandardMacros.IsValid` _capsulecomponent
    (:`Is Valid`
      (`ActorComponent.K2_DestroyComponent` _capsulecomponent))))

(fn `setDamage`
  (params (damage :type "Float (double-precision)") (criticalHitChance :type "Float (double-precision)") (criticalHitModifier :type "Float (double-precision)") (hitResult :type "HitResult Structure"))
  (returns (damageToApply :type "Float (double-precision)") (`wasCriticalHit?` :type Boolean))
  (locals (localDamageAmt :type "Float (double-precision)") (localIsCriticalHit :type Boolean))
  (set `local.localDamageAmt` damage)
  (`|ExecutionSequence`
    (:`then_0`
      (set `local.localIsCriticalHit` (< criticalHitChance (`KismetMathLibrary.RandomFloatInRange` 0.0 100.0)))
      (if true
        (set `local.localDamageAmt` (* (`local.localDamageAmt`) criticalHitModifier))))
    (:`then_1`
      (set `local.localDamageAmt` (* (`local.localDamageAmt`) (`PhysicalMaterial.DestructibleDamageThresholdScale` (`.PhysMat` (`GameplayStatics.BreakHitResult` hitResult))))))
    (:`then_2`
      (return (`local.localDamageAmt`) (`local.localIsCriticalHit`)))))

(fn `updateHealth`
  (params (Damage :type "Float (double-precision)"))
  (returns (`isDead?` :type Boolean))
  (locals (`localIsDead?` :type Boolean))
  (`|ExecutionSequence`
    (:`then_0`
      (if (>= Damage (`self.currentHealth`))
        (set `local.localIsDead?` true)
        (set `self.currentHealth` 0.0)
        (else
          (set `self.currentHealth` (- (`self.currentHealth`) Damage)))))
    (:`then_1`
      (return (`local.localIsDead?`)))))

(fn `UserConstructionScript`)