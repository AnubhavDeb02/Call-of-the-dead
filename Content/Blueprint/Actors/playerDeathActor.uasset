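; Player death actor that stands in for the player on death, applying a stored post-process look and a tumbling physics effect.
; On BeginPlay it copies PPSettings to its PostProcess component and hits the Cube with a random horizontal impulse at a random offset location.
; It then randomly fires either the LeftForce or RightForce impulse to vary the fall direction.
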(event `self.ReceiveBeginPlay`
  (bind _returnvalue (`KismetMathLibrary.RandomFloatInRange` -10.0 10.0))
  (bind _returnvalue_2 (`KismetMathLibrary.MakeVector` (* _returnvalue 650.0) (* _returnvalue 650.0)))
  (set `PostProcessComponent.Settings` (`self.PPSettings`) (`self.PostProcess`))
  (`PrimitiveComponent.AddImpulseAtLocation` (`self.Cube`) _returnvalue_2 _returnvalue_2 "None")
  (if (`KismetMathLibrary.RandomBool`)
    (`RadialForceComponent.FireImpulse` (`self.leftForce`))
    (else
      (`RadialForceComponent.FireImpulse` (`self.rightForce`)))))

(fn `UserConstructionScript`)