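; Base projectile actor that resolves its impact when its projectile movement component stops.
; Unless flagged as causing radius damage, it sends a damage message to the hit actor with its ammo data, critical hit modifier and hit result.
; In all cases it then hides its mesh, spawns the impact effect actor with the hit result and expires shortly afterwards.
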(event `self.ProjectileMovement.OnProjectileStop`
  (params (ImpactResult :type "HitResult Structure (by ref)"))
  (`self.projectileStop` ImpactResult))

(fn `projectileStop`
  (params (`Hit Result` :type "HitResult Structure"))
  (bind _mesh (`self.mesh`))
  (`|ExecutionSequence`
    (:`then_0`
      (if (not (`self.isCausingRadiusDamage?`))
        (message `/Game/Blueprint/Interfaces/TakeDamage.TakeDamage` (`.HitActor` (`GameplayStatics.BreakHitResult` `Hit Result`)) (`self.Ammo Data`) (`self.Critical Hit Modifier`) `Hit Result`)))
    (:`then_1`
      (`SceneComponent.SetHiddenInGame` _mesh true false)
      (`|SpawnActorFromClass` (`self.impactEffect`) (`SceneComponent.K2_GetComponentToWorld` _mesh) "AlwaysSpawn" "OverrideRootScale" null `Hit Result` true null)
      (`self.SetLifeSpan` 0.1))))

(fn `UserConstructionScript`)